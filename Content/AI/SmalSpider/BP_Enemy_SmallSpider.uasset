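; Small spider enemy that attaches a beam effect to its weapon socket and picks a random player-proximity threshold on BeginPlay.
; Helpers cover facing the player, moving forward and snapping to trace-hit surfaces using cross-product alignment, for wall crawling.
; The logic combining them with forward, down and back traces is disconnected, as is damage and death handling.
; Tick is empty, so the spider neither moves nor dies through this graph.
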(event Custom|MoveForward
  (Transformation|AddActorLocalOffset (Math|Vector|MakeVector (* (Variables|Default|GetDeltaTime) 5e+01) 0.0 0.0) false false))

(event Custom|RotateToPlayer
  (bind _returnvalue (Game|Player|GetPlayerPawn 0))
  (bind _returnvalue_2 (Transformation|GetActorLocation))
  (bind _returnvalue_3 (Transformation|GetActorLocation _returnvalue))
  (bind _returnvalue_4 (Math|Rotator|FindLookatRotation _returnvalue_2 _returnvalue_3))
  (Transformation|SetActorRotation (Math|Interpolation|RInterpTo (Transformation|GetActorRotation) (Math|Rotator|MakeRotator (.roll (Transformation|GetActorRotation)) (.pitch _returnvalue_4) (.yaw _returnvalue_4)) (Variables|Default|GetDeltaTime) 5.0)))

(event EventBeginPlay
  (Variables|Default|SetMinDistanceToPlayer (Math|Random|RandomFloatinRange 5e+02 7e+02))
  (Class|SceneComponent|Attachto (Variables|Default|GetFX_Beam) (Variables|Default|GetSpiderMesh) "S_Weapon" "SnapToTarget" true))

(event EventTick
  (params (DeltaSeconds :type Float%20%28single-precision%29)))

(fn ConstructionScript)

(fn ChangeLocation
  (params (HitResult :type Hit%20Result%20Structure))
  (bind (_bblockinghit _binitialoverlap _time _distance _location _impactpoint _normal _impactnormal) (Collision|BreakHitResult HitResult))
  (bind _returnvalue (Transformation|GetActorForwardVector))
  (bind _returnvalue_2 (Transformation|GetActorUpVector))
  (bind _returnvalue_3 (Math|Vector|CrossProduct _returnvalue _returnvalue_2))
  (bind _returnvalue_4 (Math|Vector|CrossProduct _impactnormal _returnvalue_3))
  (Transformation|SetActorLocation (+ _impactpoint (* _impactnormal 0.0)) false false)
  (Transformation|SetActorRotation (Math|Rotator|MakeRotationfromAxes _returnvalue_4 (Math|Vector|CrossProduct _impactnormal _returnvalue_4) _impactnormal)))

(fn IsNearPlayer
  (return (< (Math|Vector|VectorLength (- (Transformation|GetActorLocation) (Transformation|GetActorLocation (Game|Player|GetPlayerPawn 0)))) (Variables|Default|GetMinDistanceToPlayer))))